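; Terrorist character Blueprint that handles movement speed and firing in response to enemy detection.
; Every Tick sets the CharacterMovement max walk speed to the product of SpeedRate and SpeedVariable.
; AEnemyFound calls OnStartFire and AEnemyLost calls OnStopFire, each through its own DoOnce with no reset, so each call happens only on the first trigger.
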(event Custom|AEnemyLost
  (Utilities|FlowControl|DoOnce false
    (:Completed
      (Class|CSUEAICharacter|OnStopFire))))

(event Custom|AEnemyFound
  (Utilities|FlowControl|DoOnce false
    (:Completed
      (Class|CSUEAICharacter|OnStartFire))))

(event EventActorBeginOverlap
  (params (OtherActor :type Actor%20Object%20Reference)))

(event EventTick
  (params (DeltaSeconds :type Float%20%28single-precision%29))
  (Variables|/Script/Engine.CharacterMovementComponent|SetMaxWalkSpeed (Variables|Character|GetCharacterMovement) (* (Variables|Default|GetSpeedRate) (Variables|Default|GetSpeedVariable))))

(fn ConstructionScript)